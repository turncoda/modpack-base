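; BP_SafeZone is a box trigger that updates the player goat's safe zone when the goat enters it.
; At BeginPlay, a zero Offset defaults to the negative Z box extent, moving the point down from the root by that amount.
; On overlap, it passes BP_PlayerGoatMain a transform built from the root location, Offset, a fixed shift on all three axes and a configurable Yaw.
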(event OnComponentBeginOverlap(Box)
  (params (OverlappedComponent :type Primitive%20Component%20Object%20Reference) (OtherActor :type Actor%20Object%20Reference) (OtherComp :type Primitive%20Component%20Object%20Reference) (OtherBodyIndex :type Integer) (bFromSweep :type Boolean) (SweepResult :type Hit%20Result%20Structure%20%28by%20ref%29))
  (bind _asbp_player_goat_main (Utilities|Casting|CastToBP_PlayerGoatMain OtherActor))
  (Default|UpdateSafeZone _asbp_player_goat_main (Math|Transform|MakeTransform (+ (+ (Transformation|GetWorldLocation (Variables|Default|GetDefaultSceneRoot)) (Variables|Default|Getoffset)) (Math|Vector|MakeVector -64.0 -64.0 -64.0)) (Math|Rotator|MakeRotator 0.0 0.0 (Variables|Default|Getyaw)))))

(event EventBeginPlay
  (if (Utilities|Operators|EqualEqual :A (Variables|Default|Getoffset))
    (Variables|Default|Setoffset (Math|Vector|MakeVector 0.0 0.0 (* (.z (Variables|/Script/Engine.BoxComponent|GetBoxExtent (Variables|Default|GetBox))) -1.0)))))

(fn ConstructionScript)